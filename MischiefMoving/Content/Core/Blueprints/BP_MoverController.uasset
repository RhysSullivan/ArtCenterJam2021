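; BP_MoverController is an input controller that registers itself with a BP_Mover actor and records movement input.
; On BeginPlay it finds the BP_Mover in the level and adds itself to that actor's Players array.
; The MoveForward and MoveLeft axes pass through setter events into the MoveForward and MoveRight variables, with the left value stored unnegated as MoveRight.
; It applies no movement itself.
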(event `self.ReceiveBeginPlay`
  (bind _returnvalue (`GameplayStatics.GetActorOfClass` "/Game/Core/Blueprints/BP_Mover.BP_Mover_C"))
  (bind _output_get (set `self.Mover` _returnvalue))
  (`KismetArrayLibrary.Array_Add` (`/Game/Core/Blueprints/BP_Mover.Players` _output_get) self))

(event `InputAxis|MoveForward`
  (params (AxisValue :type "Float (single-precision)"))
  (`self.SetMoveForward` AxisValue))

(event `InputAxis|MoveLeft`
  (params (AxisValue :type "Float (single-precision)"))
  (`self.SetMoveLeft` AxisValue))

(event `SetMoveForward`
  (params (MoveForward :type "Float (double-precision)"))
  (set `self.MoveForward` MoveForward))

(event `SetMoveLeft`
  (params (MoveLeft :type "Float (double-precision)"))
  (set `self.Move Right` MoveLeft))

(fn `UserConstructionScript`)