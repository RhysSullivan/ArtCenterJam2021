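; Shared player-driven mover with frog and bear flipbook sprites, steered collectively by all entries in its Players array.
; On authority, Tick averages their inputs, snaps any non-zero result to full strength, then moves and switches walk/idle animations while game status permits.
; Tick also pins the spring arm's world X.
; Reset teleports to the starting transform, staging camera lag back up as authority updates game status.
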(event `DoWalkingAnimation`
  (`PaperFlipbookComponent.SetFlipbook` (`self.frog_walk`) "/Game/Art/Sprites/Frog/frog_walk.frog_walk")
  (`PaperFlipbookComponent.SetFlipbook` (`self.bear_walk`) "/Game/Art/Sprites/Bear/bear_walk.bear_walk"))

(event `self.ReceiveBeginPlay`
  (bind _output_get (set `self.RespawnTransform` (`self.GetTransform`)))
  (set `self.OGSpawnPoint` _output_get))

(event `DoIdleAnimation`
  (`PaperFlipbookComponent.SetFlipbook` (`self.frog_walk`) "/Game/Art/Sprites/Frog/frog_standstill_Flipbook.frog_standstill_Flipbook")
  (`PaperFlipbookComponent.SetFlipbook` (`self.bear_walk`) "/Game/Art/Sprites/Bear/bear_standstill1.bear_standstill1"))

(event `self.ReceiveTick`
  (params (DeltaSeconds :type "Float (single-precision)"))
  (`self.ClampCamera`)
  (`/Engine/EditorBlueprintResources/ActorMacros.Switch Has Authority`
    (:`Authority`
      (`self.DoMovement`))))

(event `Reset`
  (`self.ResetLevel`)
  (`/Engine/EditorBlueprintResources/ActorMacros.Switch Has Authority`
    (:`Authority`
      (`/Game/Core/Blueprints/BPF_Utils.SetGameStatus` "NewEnumerator4"))
    (:`Remote`
      _))
  (set `SpringArmComponent.CameraLagSpeed` 1.0 (`self.SpringArm`))
  (`self.K2_SetActorTransform` (`self.RespawnTransform`))
  (`KismetSystemLibrary.Delay` 2.2)
  (set `SpringArmComponent.CameraLagSpeed` 5.0 (`self.SpringArm`))
  (`KismetSystemLibrary.Delay` 0.3)
  (set `SpringArmComponent.CameraLagSpeed` 10.0 (`self.SpringArm`))
  (`/Engine/EditorBlueprintResources/ActorMacros.Switch Has Authority`
    (:`Authority`
      (`/Game/Core/Blueprints/BPF_Utils.SetGameStatus` "NewEnumerator1"))))

(fn `AdjustInputValue`
  (params (Input :type "Float (double-precision)"))
  (returns (NewVal :type "Float (double-precision)"))
  (bind _returnvalue (`KismetMathLibrary.Abs` Input))
  (if (> _returnvalue 0.7)
    (return (* (`KismetMathLibrary.SignOfFloat` Input) 1.0))
    (elif (> _returnvalue 0.0)
      (return (* (`KismetMathLibrary.SignOfFloat` Input) 1.0))
      (else
        (return 0.0)))))

(fn `ClampCamera`
  (bind _springarm (`self.SpringArm`))
  (bind (_returnvalue_x _returnvalue_y _returnvalue_z) (`KismetMathLibrary.BreakVector` (`SceneComponent.K2_GetComponentLocation` _springarm)))
  (`SceneComponent.K2_SetWorldLocation` _springarm (`KismetMathLibrary.MakeVector` 0.0 _returnvalue_y _returnvalue_z) false false))

(fn `DoMovement`
  (bind _players (`self.Players`))
  (bind _returnvalue (`KismetMathLibrary.Conv_IntToDouble` (`KismetArrayLibrary.Array_Length` _players)))
  (set `self.RightInput` 0.0)
  (set `self.ForwardInput` 0.0)
  (for _array_element _players
    (set `self.ForwardInput` (+ (`/Game/Core/Blueprints/BP_MoverController.MoveForward` _array_element) (`self.ForwardInput`)))
    (set `self.RightInput` (+ (`/Game/Core/Blueprints/BP_MoverController.Move Right` _array_element) (`self.RightInput`))))
  (set `self.ForwardInput` (/ (`self.ForwardInput`) _returnvalue))
  (set `self.RightInput` (/ (`self.RightInput`) _returnvalue))
  (if (`|EnumEquality` (`/Game/Core/Blueprints/BPF_Utils.GetGameStatus`) "NewEnumerator2")
    (set `self.ForwardInput` (`self.AdjustInputValue` (`self.ForwardInput`)))
    (set `self.RightInput` (`self.AdjustInputValue` (`self.RightInput`)))
    (`self.AddMovementInput` (`self.GetActorRightVector`) (`self.ForwardInput`))
    (`self.AddMovementInput` (`self.GetActorForwardVector`) (`self.RightInput`))
    (if (or (!= (`self.ForwardInput`) 0.0) (!= (`self.RightInput`) 0.0))
      (`self.DoWalkingAnimation`)
      (else
        (`self.DoIdleAnimation`)))))

(fn `UserConstructionScript`)