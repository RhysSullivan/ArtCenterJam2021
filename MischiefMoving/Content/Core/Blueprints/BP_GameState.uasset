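; BP_GameState tracks the replicated match phase: Waiting for Players, Starting, In Progress or Complete.
; Its RepNotify finds BP_FinishLine and writes the phase's status text to that actor's ProgressBar widget, blanking it during play.
; Entering Starting also calls StartGame, which waits briefly, then lets only the authority advance the state to In Progress.
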(event `StartGame`
  (`KismetSystemLibrary.Delay` 3.0)
  (`/Engine/EditorBlueprintResources/ActorMacros.Switch Has Authority`
    (:`Authority`
      (set `self.GameState` "NewEnumerator2"))))

(fn `OnRep_GameState`
  (bind _returnvalue (`GameplayStatics.GetActorOfClass` "/Game/Core/Blueprints/BP_FinishLine.BP_FinishLine_C"))
  (switch `/Game/Core/Blueprints/E_GameState` (`self.GameState`)
    (:`NewEnumerator0`
      (`self.SetGameStatusText` _returnvalue "Waiting For Players"))
    (:`NewEnumerator1`
      (`self.SetGameStatusText` _returnvalue "Starting")
      (`self.StartGame`))
    (:`NewEnumerator2`
      (`self.SetGameStatusText` _returnvalue))
    (:`NewEnumerator3`
      (`self.SetGameStatusText` _returnvalue "DONE!"))))

(fn `SetGameStatusText`
  (params (FinishLineBP :type "/Game/Core/Blueprints/BP_FinishLine Object Reference") (InText :type Text))
  (bind _progressbar (`/Game/Core/Blueprints/BP_FinishLine.ProgressBar` FinishLineBP)
    (:`then`
      (`TextBlock.SetText` (`/Game/Core/Blueprints/WBP_ProgressBar.GameStatusText` _progressbar) InText))
    (:`else`)))

(fn `UserConstructionScript`)