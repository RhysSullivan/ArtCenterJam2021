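; BP_Car is a moving car obstacle that resets any BP_Mover that touches it.
; Each tick it moves along its forward vector by MovementSpeed without sweeping or scaling by delta time, so its speed depends on frame rate.
; On BeginPlay it creates a dynamic material on the car mesh and randomizes its Base color from random unit vector components.
; A Box overlap casts the other actor to BP_Mover and calls Reset.
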(event `self.ReceiveTick`
  (params (DeltaSeconds :type "Float (single-precision)"))
  (`self.K2_AddActorWorldOffset` (* (`self.GetActorForwardVector`) (`self.MovementSpeed`))))

(event `self.ReceiveBeginPlay`
  (bind (_returnvalue_x _returnvalue_y _returnvalue_z) (`KismetMathLibrary.BreakVector` (`KismetMathLibrary.RandomUnitVector`)))
  (bind _returnvalue (`PrimitiveComponent.CreateDynamicMaterialInstance` (`self.Car`) 1 "/Game/Art/Materials/Body.Body" "None"))
  (`MaterialInstanceDynamic.SetVectorParameterValue` _returnvalue "Base" (make `LinearColor` _returnvalue_x _returnvalue_y _returnvalue_z 1.0)))

(event `self.Box.OnComponentBeginOverlap`
  (params (OverlappedComponent :type "PrimitiveComponent Object Reference") (OtherActor :type "Actor Object Reference") (OtherComp :type "PrimitiveComponent Object Reference") (OtherBodyIndex :type Integer) (bFromSweep :type Boolean) (SweepResult :type "HitResult Structure (by ref)"))
  (bind _asbp_mover (cast `/Game/Core/Blueprints/BP_Mover` OtherActor))
  (`/Game/Core/Blueprints/BP_Mover.Reset` _asbp_mover))

(fn `UserConstructionScript`)