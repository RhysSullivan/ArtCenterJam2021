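; BP_ManholeCover is an obstacle that charges up over time and then triggers a placeholder explosion.
; Tick raises ChargeAmount by ChargeSpeed scaled by delta time, lerping the cover material's Color parameter from gray to red.
; Once the charge exceeds one, a DoOnce fires Explode a single time, which currently only prints a debug message.
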(event `self.ReceiveTick`
  (params (DeltaSeconds :type "Float (single-precision)"))
  (if (> (`self.ChargeAmount`) 1.0)
    (`/Engine/EditorBlueprintResources/StandardMacros.DoOnce` false
      (:`Completed`
        (`self.Explode`)))
    (else
      (bind _output_get (set `self.ChargeAmount` (+ (`self.ChargeAmount`) (* DeltaSeconds (`self.ChargeSpeed`)))))
      (bind (_returnvalue_r _returnvalue_g _returnvalue_b) (break `LinearColor` (`KismetMathLibrary.LinearColorLerp` (struct :`R` 0.380208 :`G` 0.380208 :`B` 0.380208 :`A` 1.0) (struct :`R` 1.0 :`A` 1.0) _output_get)))
      (`MeshComponent.SetVectorParameterValueOnMaterials` (`self.ManholeCover`) "Color" (`KismetMathLibrary.MakeVector` _returnvalue_r _returnvalue_g _returnvalue_b)))))

(event `Explode`
  (`KismetSystemLibrary.PrintString` "boom!"))

(fn `UserConstructionScript`)