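; BP_CarSpawner is an obstacle actor that repeatedly spawns BP_Car actors at its own transform.
; On BeginPlay it spawns one car immediately and starts a looping timer that spawns the rest, passing each its configured movement speed.
; The timer period is the base interval plus a random offset rolled once at BeginPlay, so each spawner keeps a fixed rhythm.
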(event `self.ReceiveBeginPlay`
  (bind _returnvalue (/ (`self.RandomIntervalRange`) 2.0))
  (`KismetSystemLibrary.K2_SetTimerDelegate` (delegate `SpawnCar`) (+ (`self.SpawnInterval`) (`KismetMathLibrary.RandomFloatInRange` (* _returnvalue -1.0) _returnvalue)) true)
  (`self.SpawnCar`))

(event `SpawnCar`
  (`|SpawnActorFromClass` "/Game/Core/Blueprints/Obstacles/BP_Car.BP_Car_C" (`self.GetTransform`) "Undefined" "OverrideRootScale" null (`self.CarMovementSpeed`) null))

(fn `UserConstructionScript`)