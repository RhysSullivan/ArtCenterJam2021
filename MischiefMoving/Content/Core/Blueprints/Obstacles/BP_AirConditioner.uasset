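; BP_AirConditioner is a falling obstacle that resets any BP_Mover it hits.
; Tick lowers the Cube at FallSpeed and grows the ground Plane as it nears the Plane's height, a landing indicator in place of the Cube's disabled shadow.
; Any overlap destroys the Plane and actor on the authority.
; The actor registers with fog of war on BeginPlay.
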(event `self.ReceiveBeginPlay`
  (bind (_returnvalue_x _returnvalue_y _returnvalue_z) (`KismetMathLibrary.BreakVector` (`SceneComponent.K2_GetComponentLocation` (`self.Plane`))))
  (bind (_returnvalue_x_2 _returnvalue_y_2 _returnvalue_z_2) (`KismetMathLibrary.BreakVector` (`SceneComponent.K2_GetComponentLocation` (`self.Cube`))))
  (set `self.EndHeight` _returnvalue_z)
  (set `self.StartHeight` _returnvalue_z_2)
  (`PrimitiveComponent.SetCastShadow` (`self.Cube`) false)
  (`/Game/Core/Blueprints/BPF_Utils.AddToFogOfWar` self))

(event `self.ReceiveTick`
  (params (DeltaSeconds :type "Float (single-precision)"))
  (bind (_returnvalue_x _returnvalue_y _returnvalue_z) (`KismetMathLibrary.BreakVector` (`SceneComponent.K2_GetComponentLocation` (`self.Cube`))))
  (bind _returnvalue (- _returnvalue_z (* DeltaSeconds (`self.FallSpeed`))))
  (`SceneComponent.K2_SetWorldLocation` (`self.Cube`) (`KismetMathLibrary.MakeVector` _returnvalue_x _returnvalue_y _returnvalue) false false)
  (if (not (`self.HasCollided`))
    (`SceneComponent.SetWorldScale3D` (`self.Plane`) (* (0.5 1.0 1.0) (- 1.0 (/ (- _returnvalue (`self.EndHeight`)) (- (`self.StartHeight`) (`self.EndHeight`))))))))

(event `self.CubeCollision.OnComponentBeginOverlap`
  (params (OverlappedComponent :type "PrimitiveComponent Object Reference") (OtherActor :type "Actor Object Reference") (OtherComp :type "PrimitiveComponent Object Reference") (OtherBodyIndex :type Integer) (bFromSweep :type Boolean) (SweepResult :type "HitResult Structure (by ref)"))
  (bind _asbp_mover (cast `/Game/Core/Blueprints/BP_Mover` OtherActor)
    (:`then`
      (`/Game/Core/Blueprints/BP_Mover.Reset` _asbp_mover))
    (:`CastFailed`
      _))
  (`/Engine/EditorBlueprintResources/ActorMacros.Switch Has Authority`
    (:`Authority`
      (set `self.HasCollided` true)
      (`ActorComponent.K2_DestroyComponent` (`self.Plane`))
      (`self.K2_DestroyActor` self))))

(fn `UserConstructionScript`)