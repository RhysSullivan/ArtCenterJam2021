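; BP_AirConditioner_Spawner is an obstacle spawner that periodically spawns BP_AirConditioner actors at random points inside its SpawnerSize box.
; On BeginPlay, only the authority spawns one immediately and starts a looping timer at MinimumSpawnTime.
; SpawnTimeVariance feeds the timer's initial start delay variance, so it randomizes only the first timed spawn, with later ones at a fixed interval.
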(event `self.ReceiveBeginPlay`
  (`/Engine/EditorBlueprintResources/ActorMacros.Switch Has Authority`
    (:`Authority`
      (`KismetSystemLibrary.K2_SetTimerDelegate` (delegate `SpawnAirConditioner`) (`self.MinimumSpawnTime`) true 0.0 (`self.SpawnTimeVariance`))
      (`self.SpawnAirConditioner`))))

(event `SpawnAirConditioner`
  (`|SpawnActorFromClass` "/Game/Core/Blueprints/Obstacles/BP_AirConditioner.BP_AirConditioner_C" (`KismetMathLibrary.Conv_VectorToTransform` (`KismetMathLibrary.RandomPointInBoundingBox` (`SceneComponent.K2_GetComponentLocation` (`self.SpawnerSize`)) (`BoxComponent.GetScaledBoxExtent` (`self.SpawnerSize`)))) "Undefined" "OverrideRootScale" null null))

(fn `UserConstructionScript`)