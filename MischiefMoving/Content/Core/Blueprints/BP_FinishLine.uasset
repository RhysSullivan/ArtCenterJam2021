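; BP_FinishLine is the level's finish line, which also drives the player's on-screen progress bar.
; On BeginPlay it finds the BP_Mover, records its start location and adds a WBP_ProgressBar to the viewport.
; Each Tick converts the mover's Y distance to the line into clamped progress, setting bar percent and icon spacer height.
; When the mover overlaps the Box, it calls LevelComplete on BP_Gamemode.
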(event `self.ReceiveBeginPlay`
  (bind _returnvalue (`GameplayStatics.GetActorOfClass` "/Game/Core/Blueprints/BP_Mover.BP_Mover_C"))
  (`/Engine/EditorBlueprintResources/StandardMacros.IsValid` _returnvalue
    (:`Is Valid`
      (bind _output_get (set `self.Player` _returnvalue))
      (set `self.InitialMoverLocation` (`self.K2_GetActorLocation` _output_get))
      (bind _returnvalue_2 (`|CreateWidget` "/Game/Core/Blueprints/WBP_ProgressBar.WBP_ProgressBar_C"))
      (`UserWidget.AddToViewport` _returnvalue_2 0)
      (set `self.ProgressBar` _returnvalue_2))))

(event `self.ReceiveTick`
  (params (DeltaSeconds :type "Float (single-precision)"))
  (`/Engine/EditorBlueprintResources/StandardMacros.IsValid` (`self.ProgressBar`)
    (:`Is Valid`
      (`self.Update Progress Bar`))))

(event `self.Box.OnComponentBeginOverlap`
  (params (OverlappedComponent :type "PrimitiveComponent Object Reference") (OtherActor :type "Actor Object Reference") (OtherComp :type "PrimitiveComponent Object Reference") (OtherBodyIndex :type Integer) (bFromSweep :type Boolean) (SweepResult :type "HitResult Structure (by ref)"))
  (cast `/Game/Core/Blueprints/BP_Mover` OtherActor)
  (bind _asbp_gamemode (cast `/Game/Core/Blueprints/BP_Gamemode` (`GameplayStatics.GetGameMode`)))
  (`/Game/Core/Blueprints/BP_Gamemode.LevelComplete` _asbp_gamemode))

(fn `Update Progress Bar`
  (bind _iconspacer (`/Game/Core/Blueprints/WBP_ProgressBar.IconSpacer` (`self.ProgressBar`)))
  (bind _y (.y (`SceneComponent.K2_GetComponentLocation` (`self.FinishLine`))))
  (bind _returnvalue (`KismetMathLibrary.FClamp` (- 1.0 (`KismetMathLibrary.SafeDivide` (- _y (.y (`self.K2_GetActorLocation` (`self.Player`)))) (- _y (.y (`self.InitialMoverLocation`)))))))
  (`ProgressBar.SetPercent` (`/Game/Core/Blueprints/WBP_ProgressBar.ProgressBar_140` (`self.ProgressBar`)) _returnvalue)
  (`Spacer.SetSize` _iconspacer (`KismetMathLibrary.MakeVector2D` (`KismetMathLibrary.BreakVector2D` (`Spacer.Size` _iconspacer)) (`self.CalculateProgressIconHeight` _returnvalue))))

(fn `UserConstructionScript`)