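; Blueprint utility functions for fog of war registration and access to the game status.
; AddToFogOfWar casts the player 0 pawn to BP_Player and adds the given actor to its SceneCaptureComponent2D HiddenActors list, excluding it from that capture.
; GetGameStatus and SetGameStatus read and write the GameState variable on BP_GameState through a cast of the current game state.
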(fn `AddToFogOfWar`
  (params (SelfActor :type "Actor Object Reference (by ref)"))
  (bind _asbp_player (cast `/Game/Core/Blueprints/BP_Player` (`GameplayStatics.GetPlayerPawn` null)))
  (`KismetArrayLibrary.Array_Add` (`SceneCaptureComponent.HiddenActors` (`/Game/Core/Blueprints/BP_Player.SceneCaptureComponent2D` _asbp_player)) SelfActor))

(fn `GetGameStatus`
  (returns (GameState :type "/Game/Core/Blueprints/E_GameState Enum"))
  (return (`/Game/Core/Blueprints/BP_GameState.GameState` (cast `/Game/Core/Blueprints/BP_GameState` (`GameplayStatics.GetGameState` null) :!pure true))))

(fn `SetGameStatus`
  (params (GameState :type "/Game/Core/Blueprints/E_GameState Enum" :default "NewEnumerator0"))
  (set `/Game/Core/Blueprints/BP_GameState.GameState` GameState (cast `/Game/Core/Blueprints/BP_GameState` (`GameplayStatics.GetGameState` null) :!pure true)))